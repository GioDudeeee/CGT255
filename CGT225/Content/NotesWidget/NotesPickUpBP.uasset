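; A pickup note actor that shows a note widget on screen for the first-person character to read.
; A Box overlap tracks whether the player is close enough, and NewFunction then toggles reading only while in range.
; Picking up creates NotesPickUpWidgetBP and adds it to the viewport, while putting down removes it.
; Leaving the box always puts the note down and clears the range flag.
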(event `/Game/NotesWidget/NotesPickup.NewFunction`
  (if (`self.IsCloseEnough?`)
    (`self.Toggle pickup`)))

(event `Toggle pickup`
  (if (`self.IsReading?`)
    (`self.Put down note`)
    (else
      (`self.Pickup note`))))

(event `Pickup note`
  (bind _returnvalue (`|CreateWidget` "/Game/NotesWidget/NotesPickUpWidgetBP.NotesPickUpWidgetBP_C"))
  (`UserWidget.AddToViewport` _returnvalue 0)
  (set `self.IsReading?` true))

(event `Put down note`
  (`Widget.RemoveFromParent` (stale `Pickup note` _returnvalue))
  (set `self.IsReading?` false))

(event `self.Box.OnComponentBeginOverlap`
  (params (OverlappedComponent :type "PrimitiveComponent Object Reference") (OtherActor :type "Actor Object Reference") (OtherComp :type "PrimitiveComponent Object Reference") (OtherBodyIndex :type Integer) (bFromSweep :type Boolean) (SweepResult :type "HitResult Structure (by ref)"))
  (cast `/Game/FirstPerson/Blueprints/BP_FirstPersonCharacter` OtherActor)
  (set `self.IsCloseEnough?` true))

(event `self.Box.OnComponentEndOverlap`
  (params (OverlappedComponent :type "PrimitiveComponent Object Reference") (OtherActor :type "Actor Object Reference") (OtherComp :type "PrimitiveComponent Object Reference") (OtherBodyIndex :type Integer))
  (cast `/Game/FirstPerson/Blueprints/BP_FirstPersonCharacter` OtherActor)
  (`self.Put down note`)
  (set `self.IsCloseEnough?` false))

(fn `UserConstructionScript`)